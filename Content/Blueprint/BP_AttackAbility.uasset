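; BP_AttackAbility is a gameplay ability that performs the player character's attack.
; On activation it gets player 0's BP_ThirdPersonCharacter and picks a montage from its AttackAnim array, indexed by AttackState.
; It plays that montage through a PlayMontageAndWait task and calls StartCombo on the character as the montage starts.
; The task is ended when the montage completes, which also ends the ability, or when the ability ends.
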(event Ability|EventActivateAbility
  (bind _asbp_third_person_character (Utilities|Casting|CastToBP_ThirdPersonCharacter (Game|GetPlayerCharacter 0)))
  (Variables|Default|SetCharacter _asbp_third_person_character)
  (bind _animmontage (CallFunction|CheckState))
  (bind _asynctaskproxy (|PlayMontageandWaitProxy "None" _animmontage 1.0 "None" true 1.0 0.0)
    (:then
      (Variables|Default|SetAsync%20Task _asynctaskproxy)
      (Default|StartCombo (Variables|Default|GetCharacter)))
    (:OnCompleted
      (bind _async_task (Variables|Default|GetAsync%20Task)
        (:then
          (GameplayTasks|EndTask _async_task)
          (Ability|EndAbility))
        (:else)))))

(event Ability|EventOnEndAbility
  (params (bWasCancelled :type Boolean))
  (bind _async_task (Variables|Default|GetAsync%20Task)
    (:then
      (GameplayTasks|EndTask _async_task))
    (:else)))

(fn CheckState
  (bind _character (Variables|Default|GetCharacter))
  (return (Utilities|Array|Get(acopy) (Variables|/Script/Test.TestCharacter|GetAttackAnim _character) (Math|Conversions|ToInteger(Byte) (Variables|/Game/Blueprint/Player/BP_ThirdPersonCharacter.BP_ThirdPersonCharacter_C|GetAttackState _character)))))